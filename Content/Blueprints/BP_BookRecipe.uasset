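; BP_BookRecipe is an interactable recipe book that opens the recipe book through the GM_Ingame game mode.
; Box overlap sets an in-range flag that gates Interact, though end overlap also sets it true, so it never clears.
; Item placement is always refused, and an older path that opened a tutorial book widget directly is left disconnected.
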(event OnComponentBeginOverlap(Box)
  (params (OverlappedComponent :type Primitive%20Component%20Object%20Reference) (OtherActor :type Actor%20Object%20Reference) (OtherComp :type Primitive%20Component%20Object%20Reference) (OtherBodyIndex :type Integer) (bFromSweep :type Boolean) (SweepResult :type Hit%20Result%20Structure%20%28by%20ref%29))
  (Variables|Default|SetInrange? true))

(event OnComponentEndOverlap(Box)
  (params (OverlappedComponent :type Primitive%20Component%20Object%20Reference) (OtherActor :type Actor%20Object%20Reference) (OtherComp :type Primitive%20Component%20Object%20Reference) (OtherBodyIndex :type Integer))
  (Variables|Default|SetInrange? true))

(event EventInteract
  (params (ActorRef :type Actor%20Object%20Reference))
  (if (Variables|Default|GetInrange?)
    (bind _asgm_ingame (Utilities|Casting|CastToGM_Ingame (Game|GetGameMode)))
    (Default|ActivateRecipeBook _asgm_ingame)))

(fn ConstructionScript)

(fn CanItembePlaced?
  (params (IngredientRow :type Data%20Table%20Row%20Handle%20Structure))
  (return false))