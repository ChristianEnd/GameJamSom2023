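; Order station that hands out an ingredient order and checks the mix when an interactable actor enters its box.
; The first overlap shows the order popup behind a DoOnce; later overlaps test IsMixedRightKP, which is set elsewhere.
; Success turns the cube green, clears the popup and resets the order; failure flashes a try-again widget, then turns it red.
; GetOrderIngredients only blanks the texts, and camera activation is disconnected.
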(event OnComponentBeginOverlap(Box)
  (params (OverlappedComponent :type Primitive%20Component%20Object%20Reference) (OtherActor :type Actor%20Object%20Reference) (OtherComp :type Primitive%20Component%20Object%20Reference) (OtherBodyIndex :type Integer) (bFromSweep :type Boolean) (SweepResult :type Hit%20Result%20Structure%20%28by%20ref%29))
  ;[1 1 1] Order
  (if (Utilities|DoesObjectImplementInterface OtherActor "/Game/Blueprints/Interfaces/BPI_Interact.BPI_Interact_C")
    (Utilities|FlowControl|Sequence
      (:then_0
        (CallFunction|SetCamera))
      (:then_1
        (if (Variables|Default|GetOrderGiven)
          (CallFunction|CheckOrder)
          (else
            (CallFunction|DisplayOrder)))))))

(event OnComponentEndOverlap(Box)
  (params (OverlappedComponent :type Primitive%20Component%20Object%20Reference) (OtherActor :type Actor%20Object%20Reference) (OtherComp :type Primitive%20Component%20Object%20Reference) (OtherBodyIndex :type Integer))
  ;[1 1 1] ChangeCameraToOrderAndBack
  (Components|Activation|SetActive (Variables|Default|GetCamera) false false))

(event Custom|DisplayOrder
  ;[1 1 1] InitDisplayOrder
  (bind _returnvalue (UserInterface|CreateWidget "/Game/UI/WBP_OrderPopUp.WBP_OrderPopUp_C" (Game|GetPlayerController 0) (Variables|Default|GetIngredients%20Text) (Variables|Default|GetHeader%20Text) (Variables|Default|GetDestroy)))
  (Utilities|FlowControl|DoOnce false
    (:Completed
      (bind _output_get (Variables|Default|SetActiveOrder _returnvalue))
      (UserInterface|Viewport|AddtoViewport _output_get 0)
      (Variables|Default|SetOrderGiven true))))

(event Custom|GetOrderIngredients
  ;[1 1 1] Hier dann die Infos eingeben (Text) Wird Displayed links neben dem Character
  (Variables|Default|SetHeader%20Text "")
  (Variables|Default|SetIngredients%20Text ""))

(event Custom|CheckOrder
  ;[1 1 1] CleanUIonSuccess
  (if (Variables|Default|GetIsMixedRightKP)
    (Rendering|Material|SetMaterial (Variables|Default|GetCube) 0 "/Game/Materials/M_Green.M_Green")
    (CallFunction|GenerateNewandResetBools)
    (Widget|RemovefromParent (stale Custom|DisplayOrder _returnvalue))
    (else
      ;[1 1 1] TryAgain
      (bind _returnvalue (UserInterface|CreateWidget "/Game/UI/WBP_TryAgain.WBP_TryAgain_C" (Game|GetPlayerController 0)))
      (UserInterface|Viewport|AddtoViewport _returnvalue 0)
      (Utilities|FlowControl|Delay 1.0)
      (Widget|RemovefromParent _returnvalue)
      (Rendering|Material|SetMaterial (Variables|Default|GetCube) 0 "/Game/Materials/M_Red.M_Red"))))

(event Custom|SetCamera
  ;[1 1 1] ChangeCameraToOrderAndBack
)

(event Custom|GenerateNewAndResetBools
  ;[1 1 1] Reset
  (Variables|Default|SetOrderGiven false)
  (Variables|Default|SetIsMixedRightKP false)
  (CallFunction|ResetDoOnce))

(event Custom|ResetDoOnce
  ;[1 1 1] InitDisplayOrder
  (Utilities|FlowControl|DoOnce false) ; enters at Reset
)

(fn ConstructionScript)