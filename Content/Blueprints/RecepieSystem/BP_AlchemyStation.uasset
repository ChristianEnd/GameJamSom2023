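; Alchemy station where the player places an enchantable ingredient, processes it into another ingredient and picks it up.
; A trigger box tracks player range and drives a spinning, color-changing interaction marker.
; UseTable matches the placed row's ResultID against IDs in the ingredient DataTable, then a timeline fills a widget progress bar before swapping the mesh.
; Interact returns the item through PickUpMessage when unprocessed or finished, but not mid-process.
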(event OnComponentBeginOverlap(Box)
  (params (OverlappedComponent :type Primitive%20Component%20Object%20Reference) (OtherActor :type Actor%20Object%20Reference) (OtherComp :type Primitive%20Component%20Object%20Reference) (OtherBodyIndex :type Integer) (bFromSweep :type Boolean) (SweepResult :type Hit%20Result%20Structure%20%28by%20ref%29))
  (bind _interactionmarker (Variables|Default|GetInteractionMarker))
  (Utilities|Casting|CastToBP_MainCharacter OtherActor)
  (Variables|Default|SetInRange? true)
  (if (Utilities|DoesObjectImplementInterface OtherActor "/Game/Blueprints/Interfaces/BPI_Interact.BPI_Interact_C")
    (bind _newtrack_0 (Timeline|Timeline Play)
      (:Update
        (Transformation|SetRelativeRotation _interactionmarker (Math|Rotator|MakeRotator 0.0 0.0 (Math|Float|Lerp 0.0 359.0 _newtrack_0)) false false)
        (Rendering|Material|SetMaterial _interactionmarker 0 "/Game/Materials/M_EmissionGreen.M_EmissionGreen")))))

(event OnComponentEndOverlap(Box)
  (params (OverlappedComponent :type Primitive%20Component%20Object%20Reference) (OtherActor :type Actor%20Object%20Reference) (OtherComp :type Primitive%20Component%20Object%20Reference) (OtherBodyIndex :type Integer))
  (bind _interactionmarker (Variables|Default|GetInteractionMarker))
  (Utilities|Casting|CastToBP_MainCharacter OtherActor)
  (Variables|Default|SetInRange? false)
  (if (Utilities|DoesObjectImplementInterface OtherActor "/Game/Blueprints/Interfaces/BPI_Interact.BPI_Interact_C")
    (Rendering|Material|SetMaterial _interactionmarker 0 "/Game/UI/Fonts/Outside.Outside")
    (bind _newtrack_0 (Timeline|Timeline Stop)
      (:Update
        (Transformation|SetRelativeRotation _interactionmarker (Math|Rotator|MakeRotator 0.0 0.0 (Math|Float|Lerp 0.0 359.0 _newtrack_0)) false false)
        (Rendering|Material|SetMaterial _interactionmarker 0 "/Game/Materials/M_EmissionGreen.M_EmissionGreen")))))

(event Custom|Cutting
  (bind _ingredient_row (Variables|Default|GetIngredient%20Row))
  (bind (_datatable _rowname) (Utilities|Struct|BreakDataTableRowHandle _ingredient_row))
  (Widget|SetVisibility (Variables|Default|GetProgressbar) "Visible")
  (bind _alpha (Timeline|TL_Progress PlayFromStart)
    (:Update
      (Variables|/Game/UI/WBP_Progressbar.WBP_Progressbar_C|SetProgress (Variables|Default|GetProgressbar) (Math|Float|Lerp 0.0 1e+02 _alpha)))
    (:Finished
      (Widget|SetVisibility (Variables|Default|GetProgressbar) "Hidden")
      (Variables|Default|Setready true)
      (bind _returnvalue (Utilities|GetDataTableRow _datatable _rowname)
        (:then
          (Components|StaticMesh|SetStaticMesh (Variables|Default|GetPlacedIngredient) (.Mesh (Utilities|Struct|BreakSTRUCT_Ingredients _returnvalue))))))))

(event EventBeginPlay
  (bind _aswbp_progressbar (Utilities|Casting|CastToWBP_Progressbar (UserInterface|GetUserWidgetObject (Variables|Default|GetWidget))))
  (Variables|Default|SetProgressbar _aswbp_progressbar)
  (Widget|SetVisibility (Variables|Default|GetProgressbar) "Hidden"))

(event Collision|EventActorBeginOverlap
  (params (OtherActor :type Actor%20Object%20Reference)))

(event EventTick
  (params (DeltaSeconds :type Float%20%28single-precision%29)))

(event EventUseTable
  (params (SelfRef :type Actor%20Object%20Reference))
  (bind _dataingredients (Variables|Default|GetDataIngredients))
  ;[1 1 1] Comment
  (if (Utilities|Array|ContainsItem (Collision|GetOverlappingActors (Variables|Default|GetBox) "/Script/Engine.Pawn" :!class /Script/Engine.PrimitiveComponent) (Game|GetPlayerCharacter 0))
    (if (Variables|Default|GetPlaced)
      (if (not (Variables|Default|GetInUse))
        (Variables|Default|SetInUse true)
        (bind _outrownames (DataTable|GetDataTableRowNames _dataingredients))
        (for _array_element _outrownames
          (bind _returnvalue (Utilities|GetDataTableRow _dataingredients _array_element)
            (:then
              (if (Utilities|Enum|Equal(Enum) (Variables|Default|GetResult%20ID) (.ID (Utilities|Struct|BreakSTRUCT_Ingredients _returnvalue)))
                (Variables|Default|SetIngredient%20Row (Utilities|Struct|MakeDataTableRowHandle _dataingredients _array_element))
                (CallFunction|Cutting)))))))))

(event EventPlaceItem
  (params (IngredientRow :type Data%20Table%20Row%20Handle%20Structure))
  (bind _output_get (Variables|Default|SetIngredient%20Row IngredientRow))
  ;[1 1 1] PlaceItem
  (bind _returnvalue (Utilities|GetDataTableRow (.DataTable (Utilities|Struct|BreakDataTableRowHandle _output_get)) (.RowName (Utilities|Struct|BreakDataTableRowHandle _output_get)))
    (:then
      (Utilities|IsValid (.Mesh (Utilities|Struct|BreakSTRUCT_Ingredients _returnvalue))
        (:Is%20Valid
          (Components|StaticMesh|SetStaticMesh (Variables|Default|GetPlacedIngredient) (.Mesh (Utilities|Struct|BreakSTRUCT_Ingredients _returnvalue)))
          (Variables|Default|SetResult%20ID (.ResultID (Utilities|Struct|BreakSTRUCT_Ingredients _returnvalue)))
          (Variables|Default|SetPlaced true))))))

(event EventInteract
  (params (ActorRef :type Actor%20Object%20Reference))
  ;[1 1 1] Comment
  (if (Utilities|Array|ContainsItem (Collision|GetOverlappingActors (Variables|Default|GetBox) "/Script/Engine.Pawn" :!class /Script/Engine.PrimitiveComponent) (Game|GetPlayerCharacter 0))
    (if (Variables|Default|GetPlaced)
      (if (Variables|Default|GetInUse)
        (if (Variables|Default|Getready)
          (Variables|Default|Setready false)
          (Variables|Default|SetInUse false)
          (Utilities|IsValid (.DataTable (Utilities|Struct|BreakDataTableRowHandle (Variables|Default|GetIngredient%20Row))) :!label _label
            (:Is%20Valid
              (Class|BPIInteract|PickUp(Message) ActorRef (Variables|Default|GetIngredient%20Row))
              (Components|StaticMesh|SetStaticMesh (Variables|Default|GetPlacedIngredient) 0)
              (Variables|Default|SetIngredient%20Row "")
              (Variables|Default|SetPlaced false))))
        (else
          (goto _label))))))

(fn ConstructionScript)

(fn CanItembePlaced?
  (params (IngredientRow :type Data%20Table%20Row%20Handle%20Structure))
  (bind (_datatable _rowname) (Utilities|Struct|BreakDataTableRowHandle IngredientRow))
  (if (Variables|Default|GetInRange?)
    (Utilities|IsValid _datatable
      (:Is%20Valid
        (bind _returnvalue (Utilities|GetDataTableRow _datatable _rowname)
          (:then
            (if (.Enchantable (Utilities|Struct|BreakSTRUCT_Ingredients _returnvalue))
              (Variables|Default|SetCanbeplaced? true)
              (else
                (Variables|Default|SetCanbeplaced? false)))
            (return (Variables|Default|GetCanbeplaced?))))))))