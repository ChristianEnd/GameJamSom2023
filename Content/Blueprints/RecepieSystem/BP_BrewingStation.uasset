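; Brewing station that takes up to three ingredients and produces a potion for the player to pick up.
; The third ingredient triggers a recursive recipe-table search, intended to match in any order with "Trash" as fallback, alongside a timeline-driven progress bar.
; The result ID resolves to an ingredient-table row handle, which Interact passes to the caller while the main character is in the box.
; CanItemBePlaced checks range, brewing state and the item's Brewable flag.
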(event OnComponentBeginOverlap(Box)
  (params (OverlappedComponent :type Primitive%20Component%20Object%20Reference) (OtherActor :type Actor%20Object%20Reference) (OtherComp :type Primitive%20Component%20Object%20Reference) (OtherBodyIndex :type Integer) (bFromSweep :type Boolean) (SweepResult :type Hit%20Result%20Structure%20%28by%20ref%29))
  (Utilities|Casting|CastToBP_MainCharacter OtherActor)
  (Variables|Default|SetInRange? true))

(event OnComponentEndOverlap(Box)
  (params (OverlappedComponent :type Primitive%20Component%20Object%20Reference) (OtherActor :type Actor%20Object%20Reference) (OtherComp :type Primitive%20Component%20Object%20Reference) (OtherBodyIndex :type Integer))
  (Utilities|Casting|CastToBP_MainCharacter OtherActor)
  (Variables|Default|SetInRange? false))

(event Custom|CheckRecepie
  (bind _data_recepies (Variables|Default|GetData_Recepies))
  ;[0 0 0] Checks all Recepies > if required ingredient = added ingredients > if true Set ResultPotion ID -  if false set Result potion to "Trash"
  (bind _outrownames (DataTable|GetDataTableRowNames _data_recepies))
  (bind _returnvalue (Utilities|GetDataTableRow _data_recepies (Utilities|Array|Get(acopy) _outrownames (Variables|Default|GetRecepieIndex)))
    (:then
      (if (> (Variables|Default|GetRecepieIndex) (Utilities|Array|Length _outrownames))
        (Variables|Default|SetResultPotion "Trash")
        (Variables|Default|SetRecepieIndex 0)
        (CallFunction|SetFinalPotion)
        (else
          (bind _correct_ingredients_ (CallFunction|CompareAddedIngredients "" (.1Ingredient (Utilities|Struct|BreakSTRUCT_Recepies _returnvalue)) (.2Ingredient (Utilities|Struct|BreakSTRUCT_Recepies _returnvalue)) (.3Ingredient (Utilities|Struct|BreakSTRUCT_Recepies _returnvalue))))
          (if _correct_ingredients_
            (bind _output_get (Variables|Default|SetResultPotion (.PotionName (Utilities|Struct|BreakSTRUCT_Recepies _returnvalue))))
            (Development|PrintString _output_get)
            (CallFunction|SetFinalPotion)
            (else
              (Development|PrintString "nothing found")
              (Variables|Default|SetRecepieIndex (+ (Variables|Default|GetRecepieIndex) 1))
              (CallFunction|CHeckRecepie))))))))

(event Custom|AddIngredient
  (params (AddedIngredient :type String))
  ;[0 0 0] Add Ingredient To Array - Maximum 3 - Addcounter + 1 everytime we add a Ingredient -
  (Utilities|Array|Add (Variables|Default|GetIngredients) AddedIngredient)
  (Variables|Default|SetAddCounter (+ (Variables|Default|GetAddCounter) 1))
  (if (>= (Variables|Default|GetAddCounter) 3)
    (CallFunction|CheckRecepie)
    (CallFunction|Brew)))

(event Custom|Brew
  ;[0 0 0] Brewing Progressbar
  (Variables|Default|SetBrewing true)
  (Widget|SetVisibility (Variables|Default|GetProgressbar) "Visible")
  (bind _alpha (Timeline|TL_Progress PlayFromStart)
    (:Update
      (Variables|/Game/UI/WBP_Progressbar.WBP_Progressbar_C|SetProgress (Variables|Default|GetProgressbar) _alpha))
    (:Finished
      (Widget|SetVisibility (Variables|Default|GetProgressbar) "Hidden")
      (Variables|Default|SetBrewing false))))

(event Custom|SetFinalPotion
  (bind _data_ingredient (Variables|Default|GetData_Ingredient))
  ;[0 0 0] Set Final potion
  (bind _outrownames (DataTable|GetDataTableRowNames _data_ingredient))
  (for _array_element _outrownames
    (bind _returnvalue (Utilities|GetDataTableRow _data_ingredient _array_element)
      (:then
        (if (Utilities|Enum|Equal(Enum) (.ID (Utilities|Struct|BreakSTRUCT_Ingredients _returnvalue)) (Variables|Default|GetResultPotion))
          (Variables|Default|SetIngredientRow (Utilities|Struct|MakeDataTableRowHandle _data_ingredient _array_element)))))))

(event EventBeginPlay
  (bind _aswbp_progressbar (Utilities|Casting|CastToWBP_Progressbar (UserInterface|GetUserWidgetObject (Variables|Default|GetProgress))))
  (Variables|Default|SetProgressbar _aswbp_progressbar))

(event Collision|EventActorBeginOverlap
  (params (OtherActor :type Actor%20Object%20Reference)))

(event EventTick
  (params (DeltaSeconds :type Float%20%28single-precision%29)))

(event EventPlaceItem
  (params (IngredientRow :type Data%20Table%20Row%20Handle%20Structure))
  (bind (_datatable _rowname) (Utilities|Struct|BreakDataTableRowHandle IngredientRow))
  ;[0 0 0] PlaceItem
  (if (not (>= (Variables|Default|GetAddCounter) 3))
    (bind _returnvalue (Utilities|GetDataTableRow _datatable _rowname)
      (:then
        (CallFunction|AddIngredient (.ID (Utilities|Struct|BreakSTRUCT_Ingredients _returnvalue)))))))

(event EventInteract
  (params (ActorRef :type Actor%20Object%20Reference))
  (bind _ingredientrow (Variables|Default|GetIngredientRow))
  (if (Variables|Default|GetInRange?)
    (Utilities|IsValid (.DataTable (Utilities|Struct|BreakDataTableRowHandle _ingredientrow))
      (:Is%20Valid
        (Class|BPIInteract|PickUp(Message) ActorRef _ingredientrow)))))

(fn ConstructionScript)

(fn CompareAddedIngredients
  (params (Ingredient :type String) (1 :type String) (2 :type String) (3 :type String))
  (LocalVariables|SetCheck1 true)
  (LocalVariables|SetCheck2 true)
  (LocalVariables|SetCheck3 true)
  (for _array_element (Variables|Default|GetIngredients)
    (if (and (LocalVariables|GetCheck1) (Utilities|Enum|Equal(Enum) _array_element 1))
      (LocalVariables|SetCheck1 false)
      (elif (and (LocalVariables|GetCheck2) (Utilities|Enum|Equal(Enum) _array_element 2))
        (LocalVariables|SetCheck2 false)
        (elif (and (LocalVariables|GetCheck3) (Utilities|Enum|Equal(Enum) _array_element 3))
          (LocalVariables|SetCheck3 false))))
    (if (LocalVariables|GetCheck1)
      (Variables|Default|SetCorrect%20Ingredients? false :!label _label)
      (Development|PrintString "False")
      (elif (LocalVariables|GetCheck2)
        (goto _label)
        (elif (LocalVariables|GetCheck3)
          (goto _label)
          (else
            (Variables|Default|SetCorrect%20Ingredients? true)
            (Development|PrintString "True")))))
    (return (Variables|Default|GetCorrect%20Ingredients?))))

(fn CanItembePlaced?
  (params (IngredientRow :type Data%20Table%20Row%20Handle%20Structure))
  (bind (_datatable _rowname) (Utilities|Struct|BreakDataTableRowHandle IngredientRow))
  (if (Variables|Default|GetInRange?)
    (if (Variables|Default|GetBrewing)
      (Variables|Default|SetCanbeplaced? false)
      (else
        (Utilities|IsValid _datatable
          (:Is%20Valid
            (bind _returnvalue (Utilities|GetDataTableRow _datatable _rowname)
              (:then
                (if (.Brewable (Utilities|Struct|BreakSTRUCT_Ingredients _returnvalue))
                  (Variables|Default|SetCanbeplaced? true)
                  (else
                    (Variables|Default|SetCanbeplaced? false)))))))))
    (return (Variables|Default|GetCanbeplaced?))))