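; BP_CuttingStation is a recipe-system station that holds a cuttable ingredient; no cutting logic is implemented here.
; CanItemBePlaced checks the ingredient DataTable row's Cuttable flag, while PlaceItem stores the row handle and displays its mesh without rechecking.
; Interact passes the stored handle back through the actor's PickUpMessage, then clears the station.
; Box overlaps track whether BP_MainCharacter is in range, but Interact does not check it.
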(event OnComponentBeginOverlap(Box)
  (params (OverlappedComponent :type Primitive%20Component%20Object%20Reference) (OtherActor :type Actor%20Object%20Reference) (OtherComp :type Primitive%20Component%20Object%20Reference) (OtherBodyIndex :type Integer) (bFromSweep :type Boolean) (SweepResult :type Hit%20Result%20Structure%20%28by%20ref%29))
  (Utilities|Casting|CastToBP_MainCharacter OtherActor)
  (Variables|Default|SetInRange? true))

(event OnComponentEndOverlap(Box)
  (params (OverlappedComponent :type Primitive%20Component%20Object%20Reference) (OtherActor :type Actor%20Object%20Reference) (OtherComp :type Primitive%20Component%20Object%20Reference) (OtherBodyIndex :type Integer))
  (Utilities|Casting|CastToBP_MainCharacter OtherActor)
  (Variables|Default|SetInRange? false))

(event EventBeginPlay)

(event Collision|EventActorBeginOverlap
  (params (OtherActor :type Actor%20Object%20Reference)))

(event EventTick
  (params (DeltaSeconds :type Float%20%28single-precision%29)))

(event EventPlaceItem
  (params (IngredientRow :type Data%20Table%20Row%20Handle%20Structure))
  (bind _output_get (Variables|Default|SetIngredient%20Row IngredientRow))
  (bind _returnvalue (Utilities|GetDataTableRow (.DataTable (Utilities|Struct|BreakDataTableRowHandle _output_get)) (.RowName (Utilities|Struct|BreakDataTableRowHandle _output_get)))
    (:then
      (Components|StaticMesh|SetStaticMesh (Variables|Default|GetPlacedIngredient) (.Mesh (Utilities|Struct|BreakSTRUCT_Ingredients _returnvalue))))))

(event EventInteract
  (params (ActorRef :type Actor%20Object%20Reference))
  (Utilities|IsValid (.DataTable (Utilities|Struct|BreakDataTableRowHandle (Variables|Default|GetIngredient%20Row)))
    (:Is%20Valid
      (Class|BPIInteract|PickUp(Message) ActorRef (Variables|Default|GetIngredient%20Row))
      (Components|StaticMesh|SetStaticMesh (Variables|Default|GetPlacedIngredient) 0)
      (Variables|Default|SetIngredient%20Row ""))))

(fn ConstructionScript)

(fn CanItembePlaced?
  (params (IngredientRow :type Data%20Table%20Row%20Handle%20Structure))
  (bind (_datatable _rowname) (Utilities|Struct|BreakDataTableRowHandle IngredientRow))
  (Utilities|IsValid _datatable
    (:Is%20Valid
      (bind _returnvalue (Utilities|GetDataTableRow _datatable _rowname)
        (:then
          (if (.Cuttable (Utilities|Struct|BreakSTRUCT_Ingredients _returnvalue))
            (Variables|Default|SetCanbeplaced? true)
            (else
              (Variables|Default|SetCanbeplaced? false)))
          (return (Variables|Default|GetCanbeplaced?)))))))