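; BP_Ingredient is a world pickup for the recipe system, representing one ingredient defined by a data table row handle.
; The construction script and SpawnItem both look up that row to set the ID and static mesh.
; A sphere overlap tracks whether BP_MainCharacter is in range, gating Interact, which passes the row handle through PickUpMessage and destroys the actor after a short delay.
; CanItemBePlaced always returns false.
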(event OnComponentBeginOverlap(Sphere)
  (params (OverlappedComponent :type Primitive%20Component%20Object%20Reference) (OtherActor :type Actor%20Object%20Reference) (OtherComp :type Primitive%20Component%20Object%20Reference) (OtherBodyIndex :type Integer) (bFromSweep :type Boolean) (SweepResult :type Hit%20Result%20Structure%20%28by%20ref%29))
  (bind _asbp_main_character (Utilities|Casting|CastToBP_MainCharacter OtherActor))
  (Utilities|IsValid (Variables|Default|GetPlayer)
    (:Is%20Valid
      _)
    (:Is%20Not%20Valid
      (bind _output_get (Variables|Default|SetPlayer _asbp_main_character))
      (Development|PrintString (Utilities|GetDisplayName _output_get))))
  (Variables|Default|SetInRange true))

(event OnComponentEndOverlap(Sphere)
  (params (OverlappedComponent :type Primitive%20Component%20Object%20Reference) (OtherActor :type Actor%20Object%20Reference) (OtherComp :type Primitive%20Component%20Object%20Reference) (OtherBodyIndex :type Integer))
  (Utilities|Casting|CastToBP_MainCharacter OtherActor)
  (Variables|Default|SetInRange false))

(event EventBeginPlay)

(event Collision|EventActorBeginOverlap
  (params (OtherActor :type Actor%20Object%20Reference)))

(event EventTick
  (params (DeltaSeconds :type Float%20%28single-precision%29)))

(event EventInteract
  (params (ActorRef :type Actor%20Object%20Reference))
  (if (Variables|Default|GetInRange)
    (Class|BPIInteract|PickUp(Message) ActorRef (Variables|Default|GetRowHandle))
    (Utilities|FlowControl|Delay 0.1)
    (Actor|DestroyActor)))

(event EventSpawnItem
  (params (IngredientRow :type Data%20Table%20Row%20Handle%20Structure))
  (Variables|Default|SetRowHandle IngredientRow)
  (bind _returnvalue (Utilities|GetDataTableRow (.DataTable (Utilities|Struct|BreakDataTableRowHandle (Variables|Default|GetRowHandle))) (.RowName (Utilities|Struct|BreakDataTableRowHandle (Variables|Default|GetRowHandle))))
    (:then
      (Variables|Default|SetID (.ID (Utilities|Struct|BreakSTRUCT_Ingredients _returnvalue)))
      (Components|StaticMesh|SetStaticMesh (Variables|Default|GetMesh) (.Mesh (Utilities|Struct|BreakSTRUCT_Ingredients _returnvalue))))))

(fn ConstructionScript
  (bind _rowhandle (Variables|Default|GetRowHandle))
  (bind (_datatable _rowname) (Utilities|Struct|BreakDataTableRowHandle _rowhandle))
  (bind _returnvalue (Utilities|GetDataTableRow _datatable _rowname)
    (:then
      (Variables|Default|SetID (.ID (Utilities|Struct|BreakSTRUCT_Ingredients _returnvalue)))
      (Components|StaticMesh|SetStaticMesh (Variables|Default|GetMesh) (.Mesh (Utilities|Struct|BreakSTRUCT_Ingredients _returnvalue))))))

(fn CanItembePlaced?
  (params (IngredientRow :type Data%20Table%20Row%20Handle%20Structure))
  (return false))