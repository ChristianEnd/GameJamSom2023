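; A dialogue starter Blueprint that opens a dialogue screen when an actor implementing BPI_Interact enters its box, or when ActivateDialogue is called.
; Both paths create WBP_Dialogue with the stored text and talker list, add it to the viewport, then switch the player to UI-only input with a visible cursor.
; It has no guard against repeat triggers, and CanItemBePlaced? always returns false.
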(event OnComponentBeginOverlap(Box)
  (params (OverlappedComponent :type Primitive%20Component%20Object%20Reference) (OtherActor :type Actor%20Object%20Reference) (OtherComp :type Primitive%20Component%20Object%20Reference) (OtherBodyIndex :type Integer) (bFromSweep :type Boolean) (SweepResult :type Hit%20Result%20Structure%20%28by%20ref%29))
  (bind _returnvalue (Game|GetPlayerController 0))
  (if (Utilities|DoesObjectImplementInterface OtherActor "/Game/Blueprints/Interfaces/BPI_Interact.BPI_Interact_C")
    (bind _returnvalue_2 (UserInterface|CreateWidget "/Game/UI/WBP_Dialogue.WBP_Dialogue_C" _returnvalue 1.0 0 (Variables|Default|GetFull%20Text) true 0 (Variables|Default|GetFull%20Talker%20List)))
    (bind _output_get (Variables|Default|SetDialogueWidget _returnvalue_2))
    (UserInterface|Viewport|AddtoViewport _output_get 0)
    (Input|SetInputModeUIOnly _returnvalue _output_get "DoNotLock" true)
    (Variables|/Script/Engine.PlayerController|SetbShowMouseCursor (Game|GetPlayerController 0) true)))

(event EventActivateDialogue
  (bind _returnvalue (Game|GetPlayerController 0))
  (bind _returnvalue_2 (UserInterface|CreateWidget "/Game/UI/WBP_Dialogue.WBP_Dialogue_C" _returnvalue 1.0 0 (Variables|Default|GetFull%20Text) true 0 (Variables|Default|GetFull%20Talker%20List)))
  (bind _output_get (Variables|Default|SetDialogueWidget _returnvalue_2))
  (UserInterface|Viewport|AddtoViewport _output_get 0)
  (Input|SetInputModeUIOnly _returnvalue _output_get "DoNotLock" true)
  (Variables|/Script/Engine.PlayerController|SetbShowMouseCursor (Game|GetPlayerController 0) true))

(fn ConstructionScript)

(fn CanItembePlaced?
  (params (IngredientRow :type Data%20Table%20Row%20Handle%20Structure))
  (return false))