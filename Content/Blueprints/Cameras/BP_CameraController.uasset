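; Camera controller actor that switches the player's view between five cameras as actors move through trigger volumes.
; Each of five collision components, on begin overlap, checks that the overlapping actor implements BPI_Interact and that the player character is BP_MainCharacter.
; It then blends the player controller's view target to its paired camera over a shared BlendTime, ending in a short delay that triggers nothing further.
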(event OnComponentBeginOverlap(Collision001)
  (params (OverlappedComponent :type Primitive%20Component%20Object%20Reference) (OtherActor :type Actor%20Object%20Reference) (OtherComp :type Primitive%20Component%20Object%20Reference) (OtherBodyIndex :type Integer) (bFromSweep :type Boolean) (SweepResult :type Hit%20Result%20Structure%20%28by%20ref%29))
  (if (Utilities|DoesObjectImplementInterface OtherActor "/Game/Blueprints/Interfaces/BPI_Interact.BPI_Interact_C")
    (Utilities|Casting|CastToBP_MainCharacter (Game|GetPlayerCharacter 0))
    (Game|Player|SetViewTargetwithBlend (Game|GetPlayerController 0) (Variables|Default|GetCamera001) (Variables|Default|GetBlend%20Time) "VTBlend_Linear" 0.0 false)
    (Utilities|FlowControl|Delay 0.5)))

(event OnComponentBeginOverlap(Collision003)
  (params (OverlappedComponent :type Primitive%20Component%20Object%20Reference) (OtherActor :type Actor%20Object%20Reference) (OtherComp :type Primitive%20Component%20Object%20Reference) (OtherBodyIndex :type Integer) (bFromSweep :type Boolean) (SweepResult :type Hit%20Result%20Structure%20%28by%20ref%29))
  (if (Utilities|DoesObjectImplementInterface OtherActor "/Game/Blueprints/Interfaces/BPI_Interact.BPI_Interact_C")
    (Utilities|Casting|CastToBP_MainCharacter (Game|GetPlayerCharacter 0))
    (Game|Player|SetViewTargetwithBlend (Game|GetPlayerController 0) (Variables|Default|GetCamera003) (Variables|Default|GetBlend%20Time) "VTBlend_Linear" 0.0 false)
    (Utilities|FlowControl|Delay 0.5)))

(event OnComponentBeginOverlap(Collision002)
  (params (OverlappedComponent :type Primitive%20Component%20Object%20Reference) (OtherActor :type Actor%20Object%20Reference) (OtherComp :type Primitive%20Component%20Object%20Reference) (OtherBodyIndex :type Integer) (bFromSweep :type Boolean) (SweepResult :type Hit%20Result%20Structure%20%28by%20ref%29))
  (if (Utilities|DoesObjectImplementInterface OtherActor "/Game/Blueprints/Interfaces/BPI_Interact.BPI_Interact_C")
    (Utilities|Casting|CastToBP_MainCharacter (Game|GetPlayerCharacter 0))
    (Game|Player|SetViewTargetwithBlend (Game|GetPlayerController 0) (Variables|Default|GetCamera002) (Variables|Default|GetBlend%20Time) "VTBlend_Linear" 0.0 false)
    (Utilities|FlowControl|Delay 0.5)))

(event OnComponentBeginOverlap(Collision004)
  (params (OverlappedComponent :type Primitive%20Component%20Object%20Reference) (OtherActor :type Actor%20Object%20Reference) (OtherComp :type Primitive%20Component%20Object%20Reference) (OtherBodyIndex :type Integer) (bFromSweep :type Boolean) (SweepResult :type Hit%20Result%20Structure%20%28by%20ref%29))
  (if (Utilities|DoesObjectImplementInterface OtherActor "/Game/Blueprints/Interfaces/BPI_Interact.BPI_Interact_C")
    (Utilities|Casting|CastToBP_MainCharacter (Game|GetPlayerCharacter 0))
    (Game|Player|SetViewTargetwithBlend (Game|GetPlayerController 0) (Variables|Default|GetCamera004) (Variables|Default|GetBlend%20Time) "VTBlend_Linear" 0.0 false)
    (Utilities|FlowControl|Delay 0.5)))

(event OnComponentBeginOverlap(Collision005)
  (params (OverlappedComponent :type Primitive%20Component%20Object%20Reference) (OtherActor :type Actor%20Object%20Reference) (OtherComp :type Primitive%20Component%20Object%20Reference) (OtherBodyIndex :type Integer) (bFromSweep :type Boolean) (SweepResult :type Hit%20Result%20Structure%20%28by%20ref%29))
  (if (Utilities|DoesObjectImplementInterface OtherActor "/Game/Blueprints/Interfaces/BPI_Interact.BPI_Interact_C")
    (Utilities|Casting|CastToBP_MainCharacter (Game|GetPlayerCharacter 0))
    (Game|Player|SetViewTargetwithBlend (Game|GetPlayerController 0) (Variables|Default|GetCamera005) (Variables|Default|GetBlend%20Time) "VTBlend_Linear" 0.0 false)
    (Utilities|FlowControl|Delay 0.5)))

(fn ConstructionScript)