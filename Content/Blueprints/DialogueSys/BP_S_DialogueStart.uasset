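; Dialogue starter actor that opens a scripted conversation as soon as play begins.
; BeginPlay switches the player's view to a start camera, then after a short delay creates the dialogue widget from its text and talker lists, with UI-only input and a visible cursor.
; ActivateDialogue reopens the widget directly, skipping camera and delay.
; Its CanItemBePlaced check always refuses ingredient placement.
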(event EventBeginPlay
  (bind _returnvalue (Game|GetPlayerController 0))
  (Game|Player|SetViewTargetwithBlend _returnvalue (Variables|Default|GetStartCamera) 0.0 "VTBlend_Linear" 0.0 false)
  (Utilities|FlowControl|Delay 0.2)
  (bind _returnvalue_2 (UserInterface|CreateWidget "/Game/UI/WBP_Dialogue.WBP_Dialogue_C" _returnvalue 1.0 0 (Variables|Default|GetFull%20Text) true 0 (Variables|Default|GetFull%20Talker%20List)))
  (bind _output_get (Variables|Default|SetDialogueWidget _returnvalue_2))
  (UserInterface|Viewport|AddtoViewport _output_get 0)
  (Input|SetInputModeUIOnly _returnvalue _output_get "DoNotLock" true)
  (Variables|/Script/Engine.PlayerController|SetbShowMouseCursor (Game|GetPlayerController 0) true))

(event EventActivateDialogue
  (bind _returnvalue (Game|GetPlayerController 0))
  (bind _returnvalue_2 (UserInterface|CreateWidget "/Game/UI/WBP_Dialogue.WBP_Dialogue_C" _returnvalue 1.0 0 (Variables|Default|GetFull%20Text) true 0 (Variables|Default|GetFull%20Talker%20List)))
  (bind _output_get (Variables|Default|SetDialogueWidget _returnvalue_2))
  (UserInterface|Viewport|AddtoViewport _output_get 0)
  (Input|SetInputModeUIOnly _returnvalue _output_get "DoNotLock" true)
  (Variables|/Script/Engine.PlayerController|SetbShowMouseCursor (Game|GetPlayerController 0) true))

(fn ConstructionScript)

(fn CanItembePlaced?
  (params (IngredientRow :type Data%20Table%20Row%20Handle%20Structure))
  (return false))